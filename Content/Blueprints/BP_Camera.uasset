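; BP_Camera is a fixed-position camera actor that becomes the first player's view target at BeginPlay and turns to follow a dancer.
; The construction script caches the BP_Dancer_AbstractOmid actor found in the level.
; Each tick, it computes a look-at rotation to the Hips socket on the dancer's HumanoidCharacter, applying yaw and roll while holding a constant downward pitch.
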(event EventBeginPlay
  (Game|Player|SetViewTargetwithBlend (Game|GetPlayerController 0) self 0.0 "VTBlend_Linear" 0.0 false))

(event Collision|EventActorBeginOverlap
  (params (OtherActor :type Actor%20Object%20Reference)))

(event EventTick
  (params (DeltaSeconds :type Float%20%28single-precision%29))
  (bind _returnvalue (Transformation|GetActorLocation))
  (bind _dancer_obj (Variables|Default|GetDancer%20Obj))
  (bind _humanoid_character (Variables|/Game/Blueprints/BP_Dancer.BP_Dancer_C|GetHumanoid_Character _dancer_obj))
  (bind _returnvalue_2 (Transformation|GetSocketLocation _humanoid_character "Hips"))
  (bind _returnvalue_3 (Math|Rotator|FindLookatRotation _returnvalue _returnvalue_2))
  (Transformation|SetActorRotation (Math|Rotator|MakeRotator (.roll _returnvalue_3) -12.0 (.yaw _returnvalue_3))))

(fn ConstructionScript
  (bind _returnvalue (Actor|GetActorOfClass "/Game/Blueprints/BP_Dancer_AbstractOmid.BP_Dancer_AbstractOmid_C"))
  (Variables|Default|SetDancer%20Obj _returnvalue))