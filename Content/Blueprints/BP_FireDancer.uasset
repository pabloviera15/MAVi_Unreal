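; BP_FireDancer is a humanoid dancer actor that exposes custom events to switch its visual effects: fire, lines, hand trails, point cloud and several shape-man variants.
; The construction script puts a dynamic MI_FireFx material on the body, whose OpacityLerp the line and trail events drive.
; SetCustomColor writes to the MPC_FireColor parameter collection, replacing a deprecated per-instance color path.
; A FlipFlop toggles body visibility, and EggMan also sets a KillParticles flag.
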(event Custom|Set%20Custom%20Color
  (params (Value :type Linear%20Color%20Structure))
  (Rendering|Material|SetVectorParameterValue "/Game/Materials/FireFx/MPC_FireColor.MPC_FireColor" "Color" Value :!class /Script/Engine.KismetMaterialLibrary))

(event Custom|Deactivate_FireFx
  ;[1 1 1] Activate Particles Fx
  (Components|Activation|Deactivate (Variables|Default|GetFireFx)))

(event Custom|Activate_EggMan
  (bind _ns_eggman (Variables|Default|GetNS_EggMan))
  (Components|Activation|Activate _ns_eggman true)
  (Effects|Components|ParticleSystem|SetBoolParameter _ns_eggman "KillParticles" false))

(event Custom|Deactivate_Eggman
  (bind _ns_eggman (Variables|Default|GetNS_EggMan))
  (Components|Activation|Deactivate _ns_eggman)
  (Effects|Components|ParticleSystem|SetBoolParameter _ns_eggman "KillParticles" true))

(event Custom|Activate_FireFx
  ;[1 1 1] Activate Particles Fx
  (Components|Activation|Activate (Variables|Default|GetFireFx) true))

(event Custom|Activate_PointCloud
  (Components|Activation|Activate (Variables|Default|GetNS_PointCloud) true))

(event Custom|Deactivate_PointCloud
  (Components|Activation|Deactivate (Variables|Default|GetNS_PointCloud)))

(event Custom|Activate_SquareMan
  (Components|Activation|Activate (Variables|Default|GetNS_SquareMan) true))

(event Custom|Deactivate_SquareMan
  (Components|Activation|Deactivate (Variables|Default|GetNS_SquareMan)))

(event Custom|Deactivate_ChairMan
  (Components|Activation|Deactivate (Variables|Default|GetNS_ChairMan)))

(event Custom|Activate_TriangleMan
  (Components|Activation|Activate (Variables|Default|GetNS_TriangleMan) true))

(event Custom|Deactivate_TriangleMan
  (Components|Activation|Deactivate (Variables|Default|GetNS_TriangleMan)))

(event Custom|Activate_TrailFx
  ;[1 1 1] Activate Particles Fx
  (Components|Activation|Activate (Variables|Default|GetNS_LeftHandTrail) true)
  (Rendering|Material|SetScalarParameterValue (Variables|Default|GetMaterialInstance%20Fire) "OpacityLerp" 1.0 :!class /Script/Engine.MaterialInstanceDynamic))

(event Custom|Deactivate_TrailFx
  ;[1 1 1] Activate Particles Fx
  (Components|Activation|Deactivate (Variables|Default|GetNS_RightHandTrail))
  (Rendering|Material|SetScalarParameterValue (Variables|Default|GetMaterialInstance%20Fire) "OpacityLerp" 0.0 :!class /Script/Engine.MaterialInstanceDynamic))

(event Custom|Activate_LinesFx
  (bind _ns_linesfx (Variables|Default|GetNS_LinesFx))
  ;[1 1 1] Activate Particles Fx
  (Rendering|SetVisibility _ns_linesfx true false)
  (Components|Activation|Activate _ns_linesfx true)
  (Rendering|Material|SetScalarParameterValue (Variables|Default|GetMaterialInstance%20Fire) "OpacityLerp" 1.0 :!class /Script/Engine.MaterialInstanceDynamic))

(event Custom|Deactivate_LinesFx
  (bind _ns_linesfx (Variables|Default|GetNS_LinesFx))
  ;[1 1 1] Activate Particles Fx
  (Rendering|SetVisibility _ns_linesfx false false)
  (Components|Activation|Deactivate _ns_linesfx)
  (Rendering|Material|SetScalarParameterValue (Variables|Default|GetMaterialInstance%20Fire) "OpacityLerp" 0.0 :!class /Script/Engine.MaterialInstanceDynamic))

(event Custom|Activate_ChairMan
  (Components|Activation|Activate (Variables|Default|GetNS_ChairMan) true))

(event Custom|Hide/Show_Body
  (bind _humanoid_character (Variables|Default|GetHumanoid_Character))
  ;[1 1 1] Show/Hide Body
  (Utilities|FlowControl|FlipFlop
    (:A
      (Rendering|SetVisibility _humanoid_character false false))
    (:B
      (Rendering|SetVisibility _humanoid_character true false))))

(event EventBeginPlay
  (|CallParentFunction))

(event Collision|EventActorBeginOverlap
  (params (OtherActor :type Actor%20Object%20Reference))
  (|CallParentFunction OtherActor) ; This node is disabled and will not be called.\nDrag off pins to build functionality.
)

(event EventTick
  (params (DeltaSeconds :type Float%20%28single-precision%29))
  (|CallParentFunction DeltaSeconds) ; This node is disabled and will not be called.\nDrag off pins to build functionality.
)

(fn ConstructionScript
  (bind _humanoid_character (Variables|Default|GetHumanoid_Character))
  (|CallParentFunction)
  (bind _returnvalue (Rendering|Material|CreateDynamicMaterialInstance _humanoid_character 0 "/Game/Materials/FireFx/MI_FireFx.MI_FireFx" "None" :!class /Script/Engine.PrimitiveComponent))
  (bind _output_get (Variables|Default|SetMaterialInstance%20Fire _returnvalue))
  (Rendering|Material|SetMaterial _humanoid_character 0 _output_get))