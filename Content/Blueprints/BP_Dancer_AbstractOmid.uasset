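; Dancer actor Blueprint that manages groom hair on a humanoid character, with runtime control of hair colour and arm long-hair visibility.
; The construction script creates one dynamic hair material and shares it across the character's child grooms, so SetHairColor recolours them together.
; BeginPlay writes stored group settings into components tagged "Short Hair" and their Groom Assets.
; UseLongHair flip-flops visibility of both arms' long hair.
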(event Custom|Set%20Hair%20Color
  (params (Color :type Linear%20Color%20Structure))
  (Rendering|Material|SetVectorParameterValue (Variables|Default|GetDMI_HariColor) "Color" Color :!class /Script/Engine.MaterialInstanceDynamic))

(event Custom|Use%20Long%20Hair
  (bind _l_armlonghair (Variables|Default|GetL_ArmLongHair))
  (Utilities|FlowControl|FlipFlop
    (:A
      (Rendering|SetVisibility _l_armlonghair true false))
    (:B
      (Rendering|SetVisibility _l_armlonghair false false))))

(event EventBeginPlay
  (|CallParentFunction)
  (for _array_element (Components|GetChildrenComponents (Variables|Default|GetHumanoid_Character) false)
    (if (Components|ComponentHasTag _array_element "Short Hair")
      (bind _asgroom_component (Utilities|Casting|CastToGroomComponent _array_element))
      (Variables|/Script/HairStrandsCore.GroomAsset|SetHairGroupsPhysics (Variables|/Script/HairStrandsCore.GroomComponent|GetGroomAsset _asgroom_component) (Variables|Default|GetHair%20Grups%20Physics))
      (Variables|/Script/HairStrandsCore.GroomAsset|SetHairGroupsRendering (Variables|/Script/HairStrandsCore.GroomComponent|GetGroomAsset _asgroom_component) (Variables|Default|GetHair%20Groups%20Rendering))
      (Variables|/Script/HairStrandsCore.GroomAsset|SetHairGroupsLOD (Variables|/Script/HairStrandsCore.GroomComponent|GetGroomAsset _asgroom_component) (Variables|Default|GetHair%20Groups%20LOD))
      (Variables|/Script/HairStrandsCore.GroomAsset|SetHairGroupsInterpolation (Variables|/Script/HairStrandsCore.GroomComponent|GetGroomAsset _asgroom_component) (Variables|Default|GetHair%20Groups%20Interpolation))
      (Variables|/Script/HairStrandsCore.GroomAsset|SetHairGroupsMaterials (Variables|/Script/HairStrandsCore.GroomComponent|GetGroomAsset _asgroom_component) (Variables|Default|GetHair%20Groups%20Materials))
      (Variables|/Script/HairStrandsCore.GroomComponent|SetGroomGroupsDesc _asgroom_component (Variables|Default|GetGroom%20Groups%20Desc)))))

(event Collision|EventActorBeginOverlap
  (params (OtherActor :type Actor%20Object%20Reference))
  (|CallParentFunction OtherActor) ; This node is disabled and will not be called.\nDrag off pins to build functionality.
)

(event EventTick
  (params (DeltaSeconds :type Float%20%28single-precision%29))
  (|CallParentFunction DeltaSeconds) ; This node is disabled and will not be called.\nDrag off pins to build functionality.
)

(fn ConstructionScript
  (|CallParentFunction)
  (bind _returnvalue (Rendering|Material|CreateDynamicMaterialInstance (Variables|Default|GetR_ArmLongHair) 0 "/Game/Materials/HairDefaultMaterial1_Inst.HairDefaultMaterial1_Inst" "None" :!class /Script/Engine.PrimitiveComponent))
  (Variables|Default|SetDMI_HariColor _returnvalue)
  (for _array_element (Components|GetChildrenComponents (Variables|Default|GetHumanoid_Character) false)
    (bind _asgroom_component (Utilities|Casting|CastToGroomComponent _array_element))
    (Rendering|Material|SetMaterial _asgroom_component 0 (Variables|Default|GetDMI_HariColor))))